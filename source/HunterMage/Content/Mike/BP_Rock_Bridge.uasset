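; BP_Rock_Bridge is a rock bridge actor that moves into a fixed world position, rotation and scale when ThirdPersonCharacter_ChildPier overlaps its Box.
; The overlap plays a half-speed timeline whose alpha lerps from the actor's current transform each update, rather than a cached start.
; Every update also spawns an explosion emitter at the rock and calls EnterTrigger on all BP_Bat_Path actors.
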(event `self.Box.OnComponentBeginOverlap`
  (params (OverlappedComponent :type "PrimitiveComponent Object Reference") (OtherActor :type "Actor Object Reference") (OtherComp :type "PrimitiveComponent Object Reference") (OtherBodyIndex :type Integer) (bFromSweep :type Boolean) (SweepResult :type "HitResult Structure (by ref)"))
  (bind (_returnvalue_location _returnvalue_rotation _returnvalue_scale) (`KismetMathLibrary.BreakTransform` (`self.GetTransform`)))
  (cast `/Game/PIer/ThirdPersonCharacter_ChildPier` OtherActor)
  (bind (_direction _rock_bridge) (`Timeline|Rock_Bridge_Timeline`)
    (:`Update`
      (`GameplayStatics.SpawnEmitterAtLocation` "/Game/StarterContent/Particles/P_Explosion_Rock_Bridge.P_Explosion_Rock_Bridge" _returnvalue_location _returnvalue_rotation _returnvalue_scale)
      (`TimelineComponent.SetPlayRate` (`self.Rock_Bridge_Timeline`) 0.5)
      (`self.K2_SetActorTransform` (`KismetMathLibrary.TLerp` (`self.GetTransform`) (`KismetMathLibrary.MakeTransform` (-370.0 -4040.0 110.0) (struct :`Pitch` 60.0) (2.5 2.5 2.0)) _rock_bridge))
      (bind _outactors (`GameplayStatics.GetAllActorsOfClass` "/Game/Mike/BP_Bat_Path.BP_Bat_Path_C"))
      (`/Game/Mike/BP_Bat_Path.Enter_Trigger` _outactors))))

(fn `UserConstructionScript`)