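; BP_Bat_Path is a spline path actor that moves the level's first Smoke_Cloud_Step actor along its spline.
; BeginPlay caches that actor, and Enter_Trigger plays the Bat_path timeline, whose alpha maps to distance along the spline.
; Each update sets the smoke's world location with a Z offset and a fixed rotation, ignoring spline rotation.
; On finish, it resets the timeline time and re-triggers itself to loop.
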(event `self.ReceiveBeginPlay`
  (bind _outactors (`GameplayStatics.GetAllActorsOfClass` "/Game/Mike/Smoke_Cloud_Step.Smoke_Cloud_Step_C"))
  (set `self.Smoke` (`|GetArrayItem` _outactors)))

(event `Enter_Trigger`
  (bind (_direction _newtrack_0) (`Timeline|Bat_path` :!label _label)
    (:`Update`
      (set `self.Bat_Path_Alpha` _newtrack_0)
      (`TimelineComponent.SetPlayRate` (`self.Bat_path`) 0.5)
      (`SceneComponent.K2_SetWorldLocationAndRotation` (`Actor.RootComponent` (`self.Smoke`)) (- (`SplineComponent.GetLocationAtDistanceAlongSpline` (`self.Spline`) (`KismetMathLibrary.Lerp` 0.0 (`SplineComponent.GetSplineLength` (`self.Spline`)) (`self.Bat_Path_Alpha`)) "World") (`self.Z_Offset`)) (struct :`Yaw` -90.0) false false))
    (:`Finished`
      (`self.Play_Again`)
      (`self.Enter_Trigger`))))

(event `Play_Again`
  (goto _label :!via `SetNewTime`))

(fn `UserConstructionScript`)