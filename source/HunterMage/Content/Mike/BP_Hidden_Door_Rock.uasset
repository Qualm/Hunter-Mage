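; Hidden rock door, apparently a bridge piece, that moves to a hard-coded transform when ThirdPersonCharacter_ChildPier overlaps its box.
; The overlap plays a timeline at half speed, whose RockBridge track lerps the actor from its current transform each update, so the motion compounds.
; Each update also spawns a rock explosion emitter at the actor and calls Drop on all BP_Rock_Drop actors in the level.
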(event `self.Box.OnComponentBeginOverlap`
  (params (OverlappedComponent :type "PrimitiveComponent Object Reference") (OtherActor :type "Actor Object Reference") (OtherComp :type "PrimitiveComponent Object Reference") (OtherBodyIndex :type Integer) (bFromSweep :type Boolean) (SweepResult :type "HitResult Structure (by ref)"))
  (bind (_returnvalue_location _returnvalue_rotation _returnvalue_scale) (`KismetMathLibrary.BreakTransform` (`self.GetTransform`)))
  (cast `/Game/PIer/ThirdPersonCharacter_ChildPier` OtherActor)
  (bind (_direction _rock_bridge) (`Timeline|Timeline_0`)
    (:`Update`
      (`GameplayStatics.SpawnEmitterAtLocation` "/Game/StarterContent/Particles/P_Explosion_Rock_Bridge.P_Explosion_Rock_Bridge" _returnvalue_location _returnvalue_rotation _returnvalue_scale)
      (`TimelineComponent.SetPlayRate` (`self.Timeline_0`) 0.5)
      (`self.K2_SetActorTransform` (`KismetMathLibrary.TLerp` (`self.GetTransform`) (`KismetMathLibrary.MakeTransform` (4140.0 -7650.0 270.0) (struct :`Pitch` 60.0 :`Yaw` 1000.0) (1.0 1.0 1.0)) _rock_bridge))
      (bind _outactors (`GameplayStatics.GetAllActorsOfClass` "/Game/Mike/BP_Rock_Drop.BP_Rock_Drop_C"))
      (`/Game/Mike/BP_Rock_Drop.Drop` _outactors))))

(fn `UserConstructionScript`)